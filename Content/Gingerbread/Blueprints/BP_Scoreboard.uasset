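; BP_Scoreboard is a text display actor that shows how many BP_Lightbulb pickups remain to collect.
; On BeginPlay it binds to the OnDestroyed event of every lightbulb in the level and shows the initial count.
; Updates recount the bulbs, with an offset to discount the one being destroyed, and announce when all are found.
; The construction script applies DefaultText to the TextRender for editor preview.
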(event `self.ReceiveBeginPlay`
  (`self.RegisterBulbs`)
  (`self.UpdateBulbCountText` 0))

(fn `OnBulbCollected`
  (params (Object :type "Actor Object Reference"))
  (`self.UpdateBulbCountText` 1))

(fn `RegisterBulbs`
  (bind _outactors (`GameplayStatics.GetAllActorsOfClass` "/Game/Gingerbread/Blueprints/BP_Lightbulb.BP_Lightbulb_C"))
  (for _array_element _outactors
    (add `self.OnDestroyed` _array_element (`|CreateDelegate` :!event `OnBulbCollected`))))

(fn `SetText`
  (params (Message :type Text))
  (bind _output_get (set `self.DefaultText` Message))
  (`TextRenderComponent.K2_SetText` (`self.TextRender`) _output_get))

(fn `UpdateBulbCountText`
  (params (Offset :type Integer))
  (bind _outactors (`GameplayStatics.GetAllActorsOfClass` "/Game/Gingerbread/Blueprints/BP_Lightbulb.BP_Lightbulb_C"))
  (bind _returnvalue (- (`KismetArrayLibrary.Array_Length` _outactors) Offset))
  (if (== _returnvalue 0)
    (`self.SetText` "All Bulbs found!")
    (else
      (`self.SetText` (`|FormatText` "Collect {BulbCount} more bulbs!" _returnvalue)))))

(fn `UserConstructionScript`
  (`self.SetText` (`self.DefaultText`)))