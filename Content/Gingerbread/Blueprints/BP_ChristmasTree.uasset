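; BP_ChristmasTree is a tree actor that lights up once the gingerbread player has collected every bulb in the level.
; The construction script hides the LightBulbs component and its children, and BeginPlay stores the count of BP_Lightbulb actors as the target total.
; On overlap, it compares BP_ThirdPersonGingerbread's BulbCount to that total, then either shows the bulbs or prints that some remain to be found.
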(event `self.ReceiveBeginPlay`
  (bind _count (`self.GetRemainingBulbCount`))
  (set `self.TotalBulbCount` _count))

(event `self.ReceiveActorBeginOverlap`
  (params (OtherActor :type "Actor Object Reference"))
  (bind _asbp_third_person_gingerbread (cast `/Game/Gingerbread/Blueprints/BP_ThirdPersonGingerbread` OtherActor))
  (if (== (`/Game/Gingerbread/Blueprints/BP_ThirdPersonGingerbread.BulbCount` _asbp_third_person_gingerbread) (`self.TotalBulbCount`))
    (`self.SetBulbVisibility` true)
    (else
      (`KismetSystemLibrary.PrintString` "Still have Bulbs to find"))))

(fn `GetRemainingBulbCount`
  (returns (Count :type Integer))
  (bind _outactors (`GameplayStatics.GetAllActorsOfClass` "/Game/Gingerbread/Blueprints/BP_Lightbulb.BP_Lightbulb_C"))
  (return (`KismetArrayLibrary.Array_Length` _outactors)))

(fn `SetBulbVisibility`
  (params (IsVisible :type Boolean))
  (`SceneComponent.SetVisibility` (`self.LightBulbs`) IsVisible true))

(fn `UserConstructionScript`
  (`self.SetBulbVisibility` false))